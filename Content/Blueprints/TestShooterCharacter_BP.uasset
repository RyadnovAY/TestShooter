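; TestShooterCharacter_BP is a shooter character that drives weapon firing and reloading for multiplayer testing.
; On BeginPlay, the authority creates a Rifle_BP through WeaponManagerBP and sets it as current, with debug prints identifying host or remote.
; Fire input calls ServerFire to start or stop the weapon and print ammo.
; Reload input calls ServerReloadWeapon, which sets Reloading on FireWeapon_BP weapons and calls OnRepReloading directly.
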(event Custom|ServerReloadWeapon
  ;[1 1 1] Reload Weapon
  (bind _asfire_weapon_bp (Utilities|Casting|CastToFireWeapon_BP (Variables|/Script/TestShooter.WeaponManager|GetCurrentWeapon (Variables|Default|GetWeaponManager_BP))))
  (if true
    (Variables|/Script/TestShooter.FireWeapon|SetReloading _asfire_weapon_bp true)
    (Class|FireWeapon|OnRepReloading _asfire_weapon_bp)))

(event Custom|Server%20Fire
  (params (Activate :type Boolean))
  (bind _weaponmanager_bp (Variables|Default|GetWeaponManager_BP))
  (bind _currentweapon (Variables|/Script/TestShooter.WeaponManager|GetCurrentWeapon _weaponmanager_bp))
  ;[1 1 1] Weapon Fire (client - server)
  (if Activate
    (Class|Weapon|UseWeapon _currentweapon)
    (Development|PrintString (Utilities|String|Append (Utilities|String|ToString(Integer) (Variables|/Script/TestShooter.Weapon|GetCurrentAmmo _currentweapon)) "|" (Utilities|String|ToString(Integer) (Variables|/Script/TestShooter.Weapon|GetTotalAmmo _currentweapon))) true true "(R=1.000000,G=0.000000,B=0.030653,A=1.000000)")
    (else
      (Class|Weapon|StopUseWeapon _currentweapon))))

(event EventBeginPlay
  (Networking|SwitchHasAuthority
    (:Authority
      (bind _returnvalue (Class|WeaponManager|CreateWeapon (Variables|Default|GetWeaponManager_BP) "/Game/Blueprints/Weapons/Rifle_BP.Rifle_BP_C"))
      (Variables|/Script/TestShooter.WeaponManager|SetCurrentWeapon (Variables|Default|GetWeaponManager_BP) _returnvalue)
      (Development|PrintString "ServerHosted" true true "(R=0.353154,G=1.000000,B=0.257196,A=1.000000)" 2e+01))
    (:Remote
      (Development|PrintString "JoinGame" true true "(R=1.000000,G=0.979058,B=0.121041,A=1.000000)" 2e+01))))

(event Input|ActionEvents|InputActionFire
  (params (Key :type Key%20Structure :default "None"))
  ;[1 1 1] Weapon Fire (client - server)
  (:Pressed
    (CallFunction|ServerFire true))
  (:Released
    (CallFunction|ServerFire false)))

(event Input|ActionEvents|InputActionReload
  (params (Key :type Key%20Structure :default "None"))
  ;[1 1 1] Reload Weapon
  (:Pressed
    (Utilities|Casting|CastToFireWeapon_BP (Variables|/Script/TestShooter.WeaponManager|GetCurrentWeapon (Variables|Default|GetWeaponManager_BP)))
    (CallFunction|ServerReloadWeapon)))

(fn ConstructionScript)